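; BP_VRController is a test VR input Blueprint that fires player bullets from the camera.
; Both trigger actions share one path that spawns a Bullet at the camera manager's location, flags it as the player's, launches it along the view direction and plays a rifle sound.
; Aim follows the camera for either trigger, with no motion controller transforms used.
; A disconnected line-trace alternative that calls Boom on barricades never runs.
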(event Input|EnhancedActionEvents|EnhancedInputActionInA_Trigger_Right
  (params (ActionValue :type Boolean) (ElapsedSeconds :type Float%20%28double-precision%29) (TriggeredSeconds :type Float%20%28double-precision%29) (InputAction :type Input%20Action%20Object%20Reference :default "/Game/Interface/InA_Trigger_Right.InA_Trigger_Right"))
  (bind _returnvalue (Game|GetPlayerCameraManager 0))
  (bind _returnvalue_2 (Transformation|GetActorLocation _returnvalue))
  (bind _returnvalue_3 (Game|SpawnActorfromClass "/Game/BOTS/Bullet.Bullet_C" (Math|Conversions|ToTransform(Vector) _returnvalue_2) "Undefined" "MultiplyWithRoot" 0 0))
  (Variables|/Game/BOTS/Bullet.Bullet_C|SetPlayer_Bullet _returnvalue_3 true)
  (Variables|/Script/Engine.MovementComponent|SetVelocity (Variables|/Game/BOTS/Bullet.Bullet_C|GetProjectileMovement _returnvalue_3) (* (Transformation|GetActorForwardVector _returnvalue) 3000))
  (Audio|PlaySoundatLocation "/Game/Test/Sounds/Rifle.Rifle" _returnvalue_2 "0, 0, 0" 1.0 1.0 0.0 0 0 0 0))

(event Input|EnhancedActionEvents|EnhancedInputActionInA_Trigger_Left
  (params (ActionValue :type Boolean) (ElapsedSeconds :type Float%20%28double-precision%29) (TriggeredSeconds :type Float%20%28double-precision%29) (InputAction :type Input%20Action%20Object%20Reference :default "/Game/Interface/InA_Trigger_Left.InA_Trigger_Left"))
  (bind _returnvalue (Game|GetPlayerCameraManager 0))
  (bind _returnvalue_2 (Transformation|GetActorLocation _returnvalue))
  (bind _returnvalue_3 (Game|SpawnActorfromClass "/Game/BOTS/Bullet.Bullet_C" (Math|Conversions|ToTransform(Vector) _returnvalue_2) "Undefined" "MultiplyWithRoot" 0 0))
  (Variables|/Game/BOTS/Bullet.Bullet_C|SetPlayer_Bullet _returnvalue_3 true)
  (Variables|/Script/Engine.MovementComponent|SetVelocity (Variables|/Game/BOTS/Bullet.Bullet_C|GetProjectileMovement _returnvalue_3) (* (Transformation|GetActorForwardVector _returnvalue) 3000))
  (Audio|PlaySoundatLocation "/Game/Test/Sounds/Rifle.Rifle" _returnvalue_2 "0, 0, 0" 1.0 1.0 0.0 0 0 0 0))

(event EventBeginPlay)

(event EventTick
  (params (DeltaSeconds :type Float%20%28single-precision%29)))

(fn ConstructionScript)