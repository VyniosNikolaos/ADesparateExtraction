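; XR game mode that tracks the win and lose state by watching BOT enemies and the player's SplineVehicle.
; BeginPlay waits three seconds, then enables Tick and hides the BP_MenuEnd actor.
; Tick re-queries all BOT actors and reveals BP_MenuEnd once none remain.
; While enemies remain, a destroyed vehicle creates a WBP_YouLost widget every tick, without adding it to the viewport.
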(event EventBeginPlay
  (Utilities|FlowControl|Delay 3.0)
  (Actor|Tick|SetActorTickEnabled true)
  (bind _returnvalue (Actor|GetActorOfClass "/Game/Interface/BP_MenuEnd.BP_MenuEnd_C"))
  (Rendering|SetActorHiddenInGame _returnvalue true))

(event EventTick
  (params (DeltaSeconds :type Float%20%28single-precision%29))
  (bind _outactors (Actor|GetAllActorsOfClass "/Game/BOTS/BOT.BOT_C"))
  (bind _output_get (Variables|Default|SetEnemyActors _outactors))
  (if (Utilities|Array|IsEmpty _output_get)
    (bind _returnvalue (Actor|GetActorOfClass "/Game/Interface/BP_MenuEnd.BP_MenuEnd_C"))
    (Rendering|SetActorHiddenInGame _returnvalue false)
    (elif (Variables|/Game/Test/Vehicle/SplineVehicle.SplineVehicle_C|GetIsDestroyed (Variables|Default|GetSplineVehicle))
      (UserInterface|CreateWidget "/Game/WBP_YouLost.WBP_YouLost_C"))))

(fn ConstructionScript)